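; TargetBase_BP is a team base that takes damage and shows its remaining health on a health bar widget.
; UnitDamaged calls the parent handler with the team fixed to Player, then sets the PlayerBaseHealthBar_Widget fill to the current health fraction.
; The construction script copies the base's team to its referenced unit spawner and mirrors the actor on Y through negative scale for Enemy.
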(event EventUnitDamaged
  (params (UnitTeam :type ETeam%20Enum :default "ET_Player") (VictimTarget :type Actor%20Object%20Reference) (DamageAmount :type Float%20%28single-precision%29))
  (|CallParentFunction "ET_Player" VictimTarget DamageAmount)
  (bind _asplayer_base_health_bar_widget (Utilities|Casting|CastToPlayerBaseHealthBar_Widget (UserInterface|GetWidget (Variables|Default|GetHealthBar))))
  (Progress|SetPercent (Variables|/Game/_Game/HUD/Base/PlayerBaseHealthBar_Widget.PlayerBaseHealthBar_Widget_C|GetPlayerBase_HealthBar _asplayer_base_health_bar_widget) (/ (Variables|Default|GetHealthPoint) (Variables|Default|GetMaxHealthPoint))))

(fn ConstructionScript
  (bind _output_get (Variables|/Game/_Game/Units/UnitSpawner.UnitSpawner_C|SetTeam (Variables|BaseProperties|GetUnitSpawnerReference) (Variables|Default|GetEUnitTeam)))
  (switch Utilities|FlowControl|Switch|SwitchonETeam _output_get
    (:ET_Player
      (Transformation|SetActorScale3D (Math|Vector|MakeVector 1.0 1.0 1.0)))
    (:ET_Enemy
      (Transformation|SetActorScale3D (Math|Vector|MakeVector 1.0 -1.0 1.0)))))