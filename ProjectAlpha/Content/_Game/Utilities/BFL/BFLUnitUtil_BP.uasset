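; Blueprint function library of unit helpers for finding the player's spawner, validating damage targets and spawning attack units.
; The player spawner comes from a reference on the game instance, with an older tag-based actor search left disconnected.
; Damage targets must implement UnitDamagedInterface and not be on the given team.
; Spawning maps Basic or Heavy to an AttackUnitsDataTable row and passes it to the given spawner.
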(fn GetPlayerUnitSpawner
  (bind _as_main_game_inst_bp (Utilities|Casting|CastTo_MainGameInst_BP (Game|GetGameInstance)))
  (return (Variables|/Game/_Game/levels/_MainGameInst_BP._MainGameInst_BP_C|GetPlayerUnitSpawner _as_main_game_inst_bp)))

(fn IsActorValidforDamage
  (params (Actor :type Actor%20Object%20Reference) (UnitTeam :type ETeam%20Enum :default "ET_Player"))
  (if (Utilities|DoesObjectImplementInterface Actor "/Script/ProjectAlpha.UnitDamagedInterface")
    (LocalVariables|SetrtnValue (not (Class|UnitUtilFunctions|BFLIsActoronTeam Actor UnitTeam)))
    (else
      (LocalVariables|SetrtnValue false)))
  (return (LocalVariables|GetrtnValue)))

(fn SpawnUnitfromDataTable
  (params (UnitSpawnerRef :type Unit%20Spawner%20BP%20Object%20Reference) (RowName :type AttackUnitTypes%20Enum :default "NewEnumerator0"))
  (switch Utilities|FlowControl|Switch|SwitchonAttackUnitTypes RowName
    (:NewEnumerator0
      (LocalVariables|SetDataTableRowName "Basic"))
    (:NewEnumerator1
      (LocalVariables|SetDataTableRowName "Heavy")))
  (bind _returnvalue (Utilities|GetDataTableRow "/Game/_Game/DataTable/AttackUnitsDataTable.AttackUnitsDataTable" (LocalVariables|GetDataTableRowName))
    (:then
      (Default|CallSpawnAttackUnit UnitSpawnerRef _returnvalue)
      (return))))