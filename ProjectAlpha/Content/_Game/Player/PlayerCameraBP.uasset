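; Player camera actor that edge-scrolls horizontally along world X according to the mouse's position on screen.
; BeginPlay adds an Enhanced Input mapping context on the default player controller.
; GetMousePosition converts viewport mouse X to a -1 to 1 range, zeroing and offsetting it by a dead zone.
; The MouseX event offsets the actor by GetMouseSpeed, clamping the resulting position within symmetric bounds.
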(event EventBeginPlay
  (Utilities|FlowControl|Sequence
    (:then_0
      (bind _asdefault_player_controller (Utilities|Casting|CastToDefaultPlayerController (Game|GetPlayerController 0)))
      (Input|AddMappingContext (PlayerController|LocalPlayerSubsystems|GetEnhancedInputLocalPlayerSubsystem _asdefault_player_controller) 0 0 "(bIgnoreAllPressedKeysUntilRelease=True,bForceImmediately=False)"))))

(event Input|MouseEvents|MouseX
  (params (AxisValue :type Float%20%28single-precision%29))
  (bind _bounds (Variables|Camera|GetBounds))
  (Transformation|AddActorWorldOffset (Math|Vector|MakeVector (- (Math|Float|Clamp(Float) (+ (.x (Transformation|GetActorLocation)) (Class|PlayerCamaera|GetMouseSpeed (Variables|Camera|GetDeadZone) (Variables|Camera|GetscrollSpeed) (Variables|Camera|GetBounds))) (* _bounds -1.0) _bounds) (.x (Transformation|GetActorLocation))) 0.0 0.0)))

(fn ConstructionScript)

(fn GetMousePosition
  (params (DeadZoneAmount :type Float%20%28double-precision%29))
  (LocalVariables|SetDZAmount DeadZoneAmount)
  (LocalVariables|SetNormalizedPosition (* (- (/ (.LocationX (Game|Player|GetMousePosition (Game|GetPlayerController 0))) (.x (Viewport|GetViewportSize))) 0.5) 2.0))
  (if (and (< (LocalVariables|GetNormalizedPosition) (LocalVariables|GetDZAmount)) (> (LocalVariables|GetNormalizedPosition) (* (LocalVariables|GetDZAmount) -1.0)))
    ;[1 1 1] if (-DZ < mouse < DZ)
    (LocalVariables|SetReturnPosition 0.0)
    (elif (> (LocalVariables|GetNormalizedPosition) (LocalVariables|GetDZAmount))
      ;[1 1 1] If (DZ < mouse)
      (LocalVariables|SetReturnPosition (- (LocalVariables|GetNormalizedPosition) (LocalVariables|GetDZAmount)))
      (else
        ;[1 1 1] if (mouse < -DZ)
        (LocalVariables|SetReturnPosition (+ (LocalVariables|GetNormalizedPosition) (LocalVariables|GetDZAmount))))))
  (return (LocalVariables|GetReturnPosition)))