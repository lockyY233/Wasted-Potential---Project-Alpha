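; Base defense unit that automatically fires projectiles while a target is inside its detection area.
; Overlap with a TargetTemp_BP starts a delayed fire loop, gated by ShouldFire so additional arrivals don't stack shots, with a delay of AttackSpeed divided by 60.
; End overlap rechecks remaining targets so the loop stops once the area is empty.
; SpawnProjectile launches BaseDefenseProjectile_BP from a rotated offset along the unit's facing plus launch pitch.
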(event OnComponentBeginOverlap(TargetDetection)
  (params (OverlappedComponent :type Primitive%20Component%20Object%20Reference) (OtherActor :type Actor%20Object%20Reference) (OtherComp :type Primitive%20Component%20Object%20Reference) (OtherBodyIndex :type Integer) (bFromSweep :type Boolean) (SweepResult :type Hit%20Result%20Structure%20%28by%20ref%29))
  ;[1 1 1] When Component Begin Overlap
  (Utilities|Casting|CastToTargetTemp_BP OtherActor) ; check is target is valid
  (Variables|Default|SetIsTargetInRange true)
  ;[1 1 1] loop for keep spawning projectiles
  (if (Variables|Default|GetShouldFire) :!label _label
    (CallFunction|SpawnProjectile)
    ;;[1 1 1] Should Fire ensures no spam fires for every target that enters the area
    (Variables|Default|SetShouldFire false)
    ;;[1 1 1] Attach Speed ( in bpm)
    (Utilities|FlowControl|Delay (/ (Variables|Default|GetAttackSpeed) 6e+01))
    (Variables|Default|SetShouldFire true)
    ;;[1 1 1] if target is still in range, keep spawning projectiles
    (if (Variables|Default|GetIsTargetInRange)
      (goto _label))))

(event OnComponentEndOverlap(TargetDetection)
  (params (OverlappedComponent :type Primitive%20Component%20Object%20Reference) (OtherActor :type Actor%20Object%20Reference) (OtherComp :type Primitive%20Component%20Object%20Reference) (OtherBodyIndex :type Integer))
  ;[1 1 1] End the loop but wait for the delay
  (Utilities|Casting|CastToTargetTemp_BP OtherActor)
  ;[1 1 1] Active when a target destroyed, ensures that IsTargetInRange bool is correct
  (Variables|Default|SetIsTargetInRange (> (Utilities|Array|Length (Collision|GetOverlappingActors (Variables|Default|GetTargetDetection) "/Game/_Game/Units/Target/TargetTemp_BP.TargetTemp_BP_C" :!class /Script/Engine.PrimitiveComponent)) 0)))

(fn ConstructionScript)

(fn SpawnProjectile
  (bind _returnvalue (Transformation|GetActorRotation))
  (bind (_roll _pitch _yaw) (Math|Rotator|BreakRotator _returnvalue))
  (Game|SpawnActorfromClass "/Game/_Game/Units/Defense/BaseDefenseProjectile_BP.BaseDefenseProjectile_BP_C" (Math|Transform|MakeTransform (+ (Transformation|GetActorLocation) (Math|Vector|RotateVector (Variables|Projectile|GetProjectileOffset) _returnvalue)) (Math|Rotator|MakeRotator _roll (+ _pitch (Variables|Projectile|GetLaunchPitch)) _yaw) "1.000000,1.000000,1.000000") "Undefined" 0 (Variables|Projectile|GetProjectileSpeed) 0))