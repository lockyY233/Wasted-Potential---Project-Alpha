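; Base attack unit Blueprint that walks forward and stops to fight DebugTarget_BP actors, with placeholder weapon visuals and damage.
; On BeginPlay it hides the weapon and line-traces to snap itself onto the ground.
; Tick moves it along its forward vector until a sphere overlap stores the target and halts it.
; It then shows the weapon and runs a delayed attack loop that only prints, resuming movement after the overlap ends.
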(event OnComponentBeginOverlap(Sphere)
  (params (OverlappedComponent :type Primitive%20Component%20Object%20Reference) (OtherActor :type Actor%20Object%20Reference) (OtherComp :type Primitive%20Component%20Object%20Reference) (OtherBodyIndex :type Integer) (bFromSweep :type Boolean) (SweepResult :type Hit%20Result%20Structure%20%28by%20ref%29))
  (bind _astarget_temp_bp (Utilities|Casting|CastToDebugTarget_BP OtherActor))
  (Variables|Movement|SetbMoving false)
  (Variables|Attack|SetbWeapon true)
  (Variables|Attack|SetTargetObject _astarget_temp_bp))

(event OnComponentEndOverlap(Sphere)
  (params (OverlappedComponent :type Primitive%20Component%20Object%20Reference) (OtherActor :type Actor%20Object%20Reference) (OtherComp :type Primitive%20Component%20Object%20Reference) (OtherBodyIndex :type Integer))
  (Utilities|Casting|CastToDebugTarget_BP OtherActor)
  ;[1 1 1] replace with animation in the future
  (Utilities|FlowControl|Delay 1.0)
  (Rendering|SetVisibility (Variables|Default|GetWeapon) false false)
  (Variables|Movement|SetbMoving true)
  (Variables|Attack|SetbWeapon false))

(event EventTick
  (params (DeltaSeconds :type Float%20%28single-precision%29))
  (if (Variables|Movement|GetbMoving)
    ;[1 1 1] Interp to movement
    (Transformation|SetActorLocation (+ (* (Variables|Movement|Getspeed) (Transformation|GetActorForwardVector)) (Transformation|GetActorLocation)) false false)
    (elif (Variables|Attack|GetbWeapon)
      ;[1 1 1] Draw Weapon (replace this with animation in the future)
      (Utilities|FlowControl|Delay 0.2)
      (Rendering|SetVisibility (Variables|Default|GetWeapon) true false)
      (Variables|Attack|SetbWeapon false)
      (else
        ;[1 1 1] Damage Loop
        (Utilities|IsValid (Variables|Attack|GetTargetObject) :!label _label
          (:Is%20Valid
            (Utilities|FlowControl|Delay (Variables|Attack|GetDamageSpeed))
            ;;[1 1 1] Damage target
            (Development|PrintString "attacking")
            (goto _label))
          (:Is%20Not%20Valid
            (Development|PrintString "target is not valid")))))))

(event EventBeginPlay
  (bind _returnvalue (Transformation|GetActorLocation))
  (bind (_x _y) (Class|KismetMathLibrary|BreakVector3f _returnvalue))
  ;[1 1 1] replace with animation in the future
  (Rendering|SetVisibility (Variables|Default|GetWeapon) false false)
  ;[1 1 1] line trace to snap the actor on ground
  (bind _outhit (Collision|LineTraceByChannel _returnvalue (Math|Vector|MakeVector _x _y -3e+02) "TraceTypeQuery1" false 0 "ForDuration"))
  (Transformation|SetActorLocation (Math|Vector|MakeVector (.X (Class|KismetMathLibrary|BreakVector3f (.location _outhit))) (.Y (Class|KismetMathLibrary|BreakVector3f (.location _outhit))) (+ (.Z (Class|KismetMathLibrary|BreakVector3f (.location _outhit))) (.z (.BoxExtent (Collision|GetComponentBounds (Variables|Default|GetBodyMesh)))))) false false))

(fn ConstructionScript
  (Variables|Movement|SetbMoving true))